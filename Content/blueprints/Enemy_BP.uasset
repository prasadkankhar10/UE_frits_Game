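; Enemy Blueprint that animates its body vertically on a timeline, attacks the player on sight and is destroyed when health runs out.
; Pawn sensing starts actor rotation toward the player and a looping fire timer, both stopped by a retriggerable delay after sightings cease.
; Each shot line-traces forward with random upward offset, applies damage to the hit actor and briefly swaps two particle components' systems.
; Attack, hurt and death play sounds.
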(event OnSeePawn(PawnSensing)
  (params (Pawn :type Pawn%20Object%20Reference))
  ;[1 0.5672 0] Enemy Shoot
  (CallFunction|EnemyShoot)
  (Variables|Default|SetShoutRoadtoPlay true)
  (Utilities|FlowControl|RetriggerableDelay 4.0)
  (Variables|Default|SetShoutRoadtoPlay false)
  (Utilities|Time|ClearandInvalidateTimerbyHandle (Variables|Default|GetShootevent))
  (CallFunction|ResetOnce))

(event Custom|EnemyShoot
  ;[0.3088 0 1] Enmy Shoot
  (Utilities|FlowControl|DoOnce false
    (:Completed
      (bind _returnvalue (Utilities|Time|SetTimerbyEvent (delegate Custom|Shoot) (Variables|Default|GetFireRate) true))
      (Variables|Default|SetShootevent _returnvalue))))

(event Custom|Shoot
  (bind _returnvalue (Transformation|GetActorLocation))
  ;[0.3088 0 1] Enmy Shoot
  (Audio|PlaySoundatLocation "/Game/Kenny/sounds/enemy_attack.enemy_attack" _returnvalue "0, 0, 0" 1.0 1.0 0.0 0 0 0 0)
  (bind _outhit (Collision|LineTraceByChannel _returnvalue (+ (+ _returnvalue (* (Math|Vector|GetForwardVector (Transformation|GetActorRotation)) (Variables|Default|GetFireDenst))) (Math|Vector|MakeVector 0.0 0.0 (Math|Random|RandomFloatinRange 0.0 5e+02))) "TraceTypeQuery1" false 0 "None"))
  (Game|Damage|ApplyDamage (.HitActor (Collision|BreakHitResult _outhit)) 1.0 0 0)
  (Class|NiagaraComponent|SetAsset (Variables|Default|Getparit) "/Game/Pratcik/Enemy1System.Enemy1System" true)
  (Utilities|FlowControl|Delay 0.5)
  (Class|NiagaraComponent|SetAsset (Variables|Default|Getparit) "/Game/Pratcik/Enemy2System.Enemy2System" true))

(event Custom|Reset%20once
  ;[0.3088 0 1] Enmy Shoot
  (Utilities|FlowControl|DoOnce false) ; enters at Reset
)

(event EventBeginPlay
  (bind _enemybody (Variables|Default|GetEnemyBody))
  (bind _relativelocation (Variables|/Script/Engine.SceneComponent|GetRelativeLocation _enemybody))
  ;[1 0.03218 0] Eney to paly
  (bind _enemymovmate (Timeline|Timeline Play)
    (:Update
      (Transformation|SetRelativeLocation _enemybody (Math|Vector|MakeVector (.x _relativelocation) (.y _relativelocation) (Math|Float|Lerp 0.0 (Variables|Default|GetEnemyMovD) _enemymovmate)) false false))))

(event Collision|EventActorBeginOverlap
  (params (OtherActor :type Actor%20Object%20Reference)))

(event EventTick
  (params (DeltaSeconds :type Float%20%28single-precision%29))
  ;[0 0.752 1] Roate
  (if (Variables|Default|GetShoutRoadtoPlay)
    (Transformation|SetActorRotation (Math|Rotator|FindLookatRotation (Transformation|GetActorLocation) (Transformation|GetActorLocation (Game|GetPlayerCharacter 0))))))

(event Game|Damage|EventAnyDamage
  (params (Damage :type Float%20%28single-precision%29) (DamageType :type Damage%20Type%20Object%20Reference) (InstigatedBy :type Controller%20Object%20Reference) (DamageCauser :type Actor%20Object%20Reference))
  ;[1 0 0.4088] Enemy Damage
  (bind _output_get (Variables|Default|SetHealt (- (Variables|Default|GetHealt) Damage)))
  (if (<= _output_get 0.0)
    (Audio|PlaySoundatLocation "/Game/Kenny/sounds/enemy_destroy.enemy_destroy" (Transformation|GetActorLocation) "0, 0, 0" 1.0 1.0 0.0 0 0 0 0)
    (Actor|DestroyActor)
    (else
      (Audio|PlaySoundatLocation "/Game/Kenny/sounds/enemy_hurt.enemy_hurt" (Transformation|GetActorLocation) "0, 0, 0" 1.0 1.0 0.0 0 0 0 0))))

(fn ConstructionScript)